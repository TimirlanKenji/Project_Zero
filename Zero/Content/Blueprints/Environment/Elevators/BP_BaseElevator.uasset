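; Base elevator actor whose plane moves up and down when the player presses Interact.
; A box overlap with a BP_BaseCharacter enables input for player controller 0, and leaving the box disables it.
; Interact alternates through a FlipFlop between playing and reversing a timeline, which lerps the plane's world Z between two fixed absolute heights.
; On BeginPlay, the plane gets a random material from the Materials array.
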(event `self.ReceiveBeginPlay`
  ;[1 1 1] Set Material
  (`PrimitiveComponent.SetMaterial` (`self.Plane`) 0 (`|GetArrayItem` (`self.Materials`) (`KismetMathLibrary.RandomIntegerInRange` 0 2))))

(event `self.Box.OnComponentBeginOverlap`
  (params (OverlappedComponent :type "PrimitiveComponent Object Reference") (OtherActor :type "Actor Object Reference") (OtherComp :type "PrimitiveComponent Object Reference") (OtherBodyIndex :type Integer) (bFromSweep :type Boolean) (SweepResult :type "HitResult Structure (by ref)"))
  ;[1 1 1] Enable input
  (cast `/Game/Blueprints/Characters/BP_BaseCharacter` OtherActor)
  (`self.EnableInput` (`GameplayStatics.GetPlayerController` 0)))

(event `self.Box.OnComponentEndOverlap`
  (params (OverlappedComponent :type "PrimitiveComponent Object Reference") (OtherActor :type "Actor Object Reference") (OtherComp :type "PrimitiveComponent Object Reference") (OtherBodyIndex :type Integer))
  ;[1 1 1] Disable input
  (cast `/Game/Blueprints/Characters/BP_BaseCharacter` OtherActor)
  (`self.DisableInput` (`GameplayStatics.GetPlayerController` 0)))

(event `InputAction|Interact`
  (params (Key :type "Key Structure"))
  (bind (_returnvalue_x _returnvalue_y) (`KismetMathLibrary.BreakVector` (`SceneComponent.K2_GetComponentLocation` (`self.Plane`))))
  ;[1 1 1] Up and Down logic
  (:`Pressed`
    (`/Engine/EditorBlueprintResources/StandardMacros.FlipFlop`
      (:`A`
        (bind (_direction _z_value) (`Timeline|ElevatorHight` :!label _label)
          (:`Update`
            (`SceneComponent.K2_SetWorldLocation` (`self.Plane`) (`KismetMathLibrary.MakeVector` _returnvalue_x _returnvalue_y (`KismetMathLibrary.Lerp` 140.0 500.0 _z_value)) false false))))
      (:`B`
        (goto _label :!via `Reverse`)))))

(fn `UserConstructionScript`)