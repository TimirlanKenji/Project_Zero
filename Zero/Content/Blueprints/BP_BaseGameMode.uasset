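; Base game mode that respawns the player whenever their character is destroyed.
; On BeginPlay it binds to the player character's OnDestroyed, which calls the PlayerFell dispatcher, waits briefly, then runs Respawn.
; Respawn prints a message, spawns a BP_BaseCharacter at the location of a found PlayerStart and possesses it with player controller 0.
; The destroyed binding is then reapplied to the new character, so the cycle repeats.
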(event `self.ReceiveBeginPlay`
  (add `self.OnDestroyed` (`GameplayStatics.GetPlayerCharacter` 0) (delegate `OnDestroyed_Event_0`) :!label _label))

(event `OnDestroyed_Event_0` :!signature `self.OnDestroyed`
  (params (DestroyedActor :type "Actor Object Reference"))
  (`self.Player Fell`)
  (`KismetSystemLibrary.Delay` 2.0)
  (`self.Respawn` (`GameplayStatics.GetPlayerController` 0))
  (goto _label))

(fn `Respawn`
  (params (NewParam :type "Actor Object Reference"))
  (`KismetSystemLibrary.PrintString` "PLAYER RESTART! ")
  (bind _returnvalue (`GameplayStatics.GetActorOfClass` "/Script/Engine.PlayerStart"))
  (bind _returnvalue_location (`KismetMathLibrary.BreakTransform` (`self.GetTransform` _returnvalue)))
  (bind _returnvalue_2 (`|SpawnActorFromClass` "/Game/Blueprints/Characters/BP_BaseCharacter.BP_BaseCharacter_C" (`KismetMathLibrary.MakeTransform` _returnvalue_location) "Undefined" "OverrideRootScale" null null))
  (`Controller.Possess` (`GameplayStatics.GetPlayerController` 0) _returnvalue_2))

(fn `UserConstructionScript`)