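; BP_LightBase is a base light actor that exposes point light settings as variables for placing lights in levels.
; The construction script applies intensity, radius, color and shadow casting to the PointLight and fixes its intensity units to candelas.
; It also scales a Cube component and can destroy it through a flag.
; The event graph holds no active logic.
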(fn `UserConstructionScript`
  (bind _pointlight (`self.PointLight`))
  (`LightComponent.SetIntensity` _pointlight (`self.LightIntensity`))
  (`LocalLightComponent.SetAttenuationRadius` _pointlight (`self.LightRadius`))
  (`LightComponent.SetLightColor` _pointlight (`self.ColorLight`) false)
  (`LightComponentBase.SetCastShadows` _pointlight (`self.LightShadows`))
  (`LocalLightComponent.SetIntensityUnits` _pointlight "Candelas")
  (`SceneComponent.SetWorldScale3D` (`self.Cube`) (`self.CubeScale`))
  (if (`self.DestroyCube?`)
    (`ActorComponent.K2_DestroyComponent` (`self.Cube`))))